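; Troll enemy with heavy and charge melee attacks plus a ranged vomit projectile, built on inherited combat, targeting and damage functions.
; On authority, heavy and special attacks sphere-overlap in front of the troll, damaging players and launching them away and upward.
; The ranged attack spawns the projectile server-side.
; While in combat, it picks an attack by target distance, delays, then moves to the player to attack, clearing the target on failure.
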(event `/Game/_Main/Interfaces/BPI_EnemyAI.DoSphereOverlap`
  (`/Engine/EditorBlueprintResources/ActorMacros.Switch Has Authority`
    (:`Authority`
      (switch `/Game/_Main/AI/EAI_AttackTypes` (`self.F_GetAttackType`)
        (:`NewEnumerator1`
          ;[1 1 1] Heavy Attack does a Knockback
          (bind _outactors (`KismetSystemLibrary.SphereOverlapActors` (+ (`self.K2_GetActorLocation`) (* (`self.GetActorForwardVector`) 200.0)) 100.0 (`|MakeArray` "ObjectTypeQuery3" :!type "EObjectTypeQuery Enum") null (`|MakeArray` self :!type "Actor Object Reference")))
          (for _array_element _outactors
            (if (`self.ActorHasTag` _array_element "Player")
              (`self.F Get Damage` _array_element)
              (bind _ascharacter (cast `Character` _array_element :!pure true))
              (`self.LaunchCharacter` _ascharacter (* (`KismetMathLibrary.MakeVector` (.x (`KismetMathLibrary.GetDirectionUnitVector` (`self.K2_GetActorLocation`) (`self.K2_GetActorLocation` _ascharacter))) (.y (`KismetMathLibrary.GetDirectionUnitVector` (`self.K2_GetActorLocation`) (`self.K2_GetActorLocation` _ascharacter))) (+ (.z (`KismetMathLibrary.GetDirectionUnitVector` (`self.K2_GetActorLocation`) (`self.K2_GetActorLocation` _ascharacter))) 1.0)) 900.0) false false))))
        (:`NewEnumerator3`
          ;[1 1 1] Charge Attack
          (bind _outactors_2 (`KismetSystemLibrary.SphereOverlapActors` (+ (`self.K2_GetActorLocation`) (* (`self.GetActorForwardVector`) 200.0)) 100.0 (`|MakeArray` "ObjectTypeQuery3" :!type "EObjectTypeQuery Enum") null (`|MakeArray` self :!type "Actor Object Reference")))
          (for _array_element_2 _outactors_2
            (if (`self.ActorHasTag` _array_element_2 "Player")
              (`self.F Get Damage` _array_element_2)
              (bind _ascharacter_2 (cast `Character` _array_element_2 :!pure true))
              (`self.LaunchCharacter` _ascharacter_2 (* (`KismetMathLibrary.MakeVector` (.x (`KismetMathLibrary.GetDirectionUnitVector` (`self.K2_GetActorLocation`) (`self.K2_GetActorLocation` _ascharacter_2))) (.y (`KismetMathLibrary.GetDirectionUnitVector` (`self.K2_GetActorLocation`) (`self.K2_GetActorLocation` _ascharacter_2))) (+ (.z (`KismetMathLibrary.GetDirectionUnitVector` (`self.K2_GetActorLocation`) (`self.K2_GetActorLocation` _ascharacter_2))) 1.0)) 900.0) false false))))))))

(event `/Game/_Main/Interfaces/BPI_EnemyAI.ChasePlayer`
  (if (`self.F_GetCombatState`)
    (bind _length (`self.F_PickAttack` (`self.GetDistanceTo` self (`self.F_GetPlayerTarget`))))
    (`KismetSystemLibrary.Delay` _length)
    (`|AIMoveTo` self (0.0 0.0 0.0) (`self.F_GetPlayerTarget`) 70.0 true
      (:`OnSuccess`
        (`/Game/_Main/Interfaces/BPI_EnemyAI.RunAttackChoices`))
      (:`OnFail`
        (`KismetSystemLibrary.PrintString` "Failed to move towards Player, Clearing Target.")
        (`/Game/_Main/Interfaces/BPI_EnemyAI.ClearTarget`)))))

(event `/Game/_Main/Interfaces/BPI_EnemyAI.DoRangedAttack`
  (`/Engine/EditorBlueprintResources/ActorMacros.Switch Has Authority`
    (:`Authority`
      (`|SpawnActorFromClass` "/Game/_Main/AI/Troll/BP_VomitProjectile.BP_VomitProjectile_C" (`SceneComponent.K2_GetComponentToWorld` (`self.VomitSpawnPoint`)) "AlwaysSpawn" "OverrideRootScale" self (`self.RangedAttackDamage`) null))))

(fn `F_PlayDeathAnim`
  (`SkeletalMeshComponent.PlayAnimation` (`self.Mesh`) "/Game/InfinityBladeAdversaries/Enemy/Enemy_Troll/Enemy_Troll_Poison_Animation/ExoGame_Troll_Death_.ExoGame_Troll_Death_" false))

(fn `UserConstructionScript`
  (`parent.UserConstructionScript`))