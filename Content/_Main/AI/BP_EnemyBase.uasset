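; Base AI enemy character that roams around its spawn, fights a player target, and awards souls XP on death.
; Once given a target, it faces it, taunts if far, then loops chasing and distance-based attack picks with random montages played via multicast.
; Authority-only melee or sphere overlaps apply damage per attack type; ranged attack and death animation are empty hooks.
; A looping distance timer drops far targets, returning it to where combat began.
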(event `self.ReceiveBeginPlay`
  ;[1 1 1] BeginPlay: Start Roaming
  (set `self.SpawnLocation` (`self.K2_GetActorLocation`))
  (`KismetSystemLibrary.Delay` 1.0)
  (`self.SetRoaming`))

(event `Multi_PlayMontage`
  (params (InSkeletalMeshComponent :type "SkeletalMeshComponent Object Reference") (MontageToPlay :type "AnimMontage Object Reference") (StartingSection :type Name))
  (`|PlayMontage` InSkeletalMeshComponent MontageToPlay 1.0 0.0 StartingSection))

(event `self.SetRoaming`
  ;[1 1 1] Roaming
  (if (and (not (`self.IsRoaming`)) (not (`self.InCombat`)))
    (`self.F_MovementState` "NewEnumerator1")
    (`|AIMoveTo` self (`NavigationSystemV1.K2_GetRandomReachablePointInRadius` (`self.SpawnLocation`) 1000.0 null null) null 150.0
      (:`then`
        (set `self.IsRoaming` true))
      (:`OnSuccess`
        (set `self.IsRoaming` false)
        (`KismetSystemLibrary.Delay` 5.0)
        (`self.SetRoaming`)))))

(event `self.ReceiveAnyDamage`
  (params (Damage :type "Float (single-precision)") (DamageType :type "DamageType Object Reference") (InstigatedBy :type "Controller Object Reference") (DamageCauser :type "Actor Object Reference"))
  (bind _output_get (set `self.Health` (- (`self.Health`) Damage)))
  (if (<= _output_get 0.0)
    (`self.Death` DamageCauser)))

(event `self.SetPlayerTarget`
  (params (PlayerTarget :type "Actor Object Reference"))
  ;[1 1 1] Set Player Target and Rotate Towards Player
  (set `self.PlayerTarget` PlayerTarget)
  (set `self.InCombat` true)
  (set `self.IsRoaming` false)
  (`self.SetActorTickEnabled` true)
  (set `self.StartingCombatLocation` (`self.K2_GetActorLocation`))
  (`self.F_MovementState` "NewEnumerator2")
  (`self.CheckForTaunt`)
  (bind _returnvalue (`KismetSystemLibrary.K2_SetTimer` null "F_DistanceCheck" 0.5 true))
  (set `self.DistanceHandle` _returnvalue))

(event `self.ReceiveTick`
  (params (DeltaSeconds :type "Float (single-precision)"))
  (bind (_returnvalue_roll _returnvalue_pitch _returnvalue_yaw) (`KismetMathLibrary.BreakRotator` (`KismetMathLibrary.FindLookAtRotation` (`self.K2_GetActorLocation`) (`self.K2_GetActorLocation` (`self.PlayerTarget`)))))
  ;[1 1 1] Set Player Target and Rotate Towards Player
  (if (`self.InCombat`)
    (`self.PlayerTarget`
      (:`then`
        (`self.K2_SetActorRotation` (`KismetMathLibrary.MakeRotator` 0.0 0.0 _returnvalue_yaw)))
      (:`else`))))

(event `self.CheckForTaunt`
  (bind _output (`self.F_GetMontage` (`self.TauntMontage`)))
  ;[1 1 1] Taunt/Aggro
  (`Controller.StopMovement` (`self.GetController`))
  (if (>= (`self.GetDistanceTo` self (`self.PlayerTarget`)) 800.0)
    (`self.Multi_PlayMontage` (`self.Mesh`) _output)
    (bind _returnvalue (`AnimSequenceBase.GetPlayLength` _output))
    (`KismetSystemLibrary.Delay` _returnvalue)
    (`self.ChasePlayer`)
    (else
      (`self.ChasePlayer`))))

(event `self.ChasePlayer`
  ;[1 1 1] Chasing Player
  (if (`self.InCombat`)
    (`|AIMoveTo` self (0.0 0.0 0.0) (`self.PlayerTarget`) 70.0 true
      (:`OnSuccess`
        (`self.RunAttackChoices`)))))

(event `self.RunAttackChoices`
  ;[1 1 1] RunAttackChoices
  (bind _playertarget (`self.PlayerTarget`)
    (:`then`
      (bind _dead (message `/Game/_Main/Interfaces/BPI_HeroCharacter.IsDead` _playertarget))
      (if (not _dead)
        (bind _length (`self.F_PickAttack` (`self.GetDistanceTo` self (`self.PlayerTarget`))))
        (`KismetSystemLibrary.Delay` _length)
        (`self.ChasePlayer`)
        (else
          (`self.ClearTarget`))))
    (:`else`
      (`self.ClearTarget`))))

(event `self.SetMeleeCollision`
  (params (State :type Boolean))
  (bind _meleesphere (`self.MeleeSphere`))
  ;[1 1 1] SetMeleeCollision
  (if State
    (`PrimitiveComponent.SetCollisionEnabled` _meleesphere "QueryOnly")
    (else
      (`PrimitiveComponent.SetCollisionEnabled` _meleesphere "NoCollision"))))

(event `self.MeleeSphere.OnComponentBeginOverlap`
  (params (OverlappedComponent :type "PrimitiveComponent Object Reference") (OtherActor :type "Actor Object Reference") (OtherComp :type "PrimitiveComponent Object Reference") (OtherBodyIndex :type Integer) (bFromSweep :type Boolean) (SweepResult :type "HitResult Structure (by ref)"))
  (`/Engine/EditorBlueprintResources/ActorMacros.Switch Has Authority`
    (:`Authority`
      (if (`self.ActorHasTag` OtherActor "Player")
        (`self.F Get Damage` OtherActor)))))

(event `self.DoSphereOverlap`
  ;[1 1 1] DoSphereOverlap
  (`/Engine/EditorBlueprintResources/ActorMacros.Switch Has Authority`
    (:`Authority`
      (bind _outactors (`KismetSystemLibrary.SphereOverlapActors` (+ (`self.K2_GetActorLocation`) (* (`self.GetActorForwardVector`) 200.0)) 100.0 (`|MakeArray` "ObjectTypeQuery3" :!type "EObjectTypeQuery Enum") null (`|MakeArray` self :!type "Actor Object Reference")))
      (for _array_element _outactors
        (if (`self.ActorHasTag` _array_element "Player")
          (`self.F Get Damage` _array_element))))))

(event `self.DoRangedAttack`)

(event `self.Death`
  (params (DeathCause :type "Actor Object Reference"))
  (bind _charactermovement (`self.CharacterMovement`))
  ;[1 1 1] Event Death
  (if (not (`self.IsDead`))
    (set `self.IsDead` true)
    (message `/Game/_Main/Interfaces/BPI_HeroCharacter.SpawnSoulsParticle` DeathCause (`self.SoulsXPAmount`))
    (`self.Multi_DeadAnimation`)
    (`self.ClearTarget`)
    (`self.DetachFromControllerPendingDestroy`)
    (`CharacterMovementComponent.SetAvoidanceEnabled` _charactermovement false)
    (`CharacterMovementComponent.DisableMovement` _charactermovement)
    (`KismetSystemLibrary.Delay` 5.0)
    (`self.K2_DestroyActor`)))

(event `Multi_DeadAnimation`
  ;[1 1 1] Dead Animation
  (`PrimitiveComponent.SetCollisionProfileName` (`self.CapsuleComponent`) "Ragdoll" true)
  (`SkeletalMeshComponent.SetAnimationMode` (`self.Mesh`) "AnimationSingleNode")
  (`self.F_PlayDeathAnim`))

(event `self.ClearTarget`
  (bind _startingcombatlocation (`self.StartingCombatLocation`))
  ;[1 1 1] Clear Target
  (set `self.InCombat` false)
  (`self.SetActorTickEnabled` false)
  (set `self.PlayerTarget` null)
  (`/Game/_Main/AI/AIC_Enemy.ClearTarget` (cast `/Game/_Main/AI/AIC_Enemy` (`self.GetController`) :!pure true))
  (`|AIMoveTo` self _startingcombatlocation null 150.0
    (:`OnSuccess`
      (`self.SetRoaming`)
      (`self.F_MovementState` "NewEnumerator1"))
    (:`OnFail`
      (`self.K2_SetActorLocation` _startingcombatlocation)
      (`self.SetRoaming`))))

(fn `F Get Damage`
  (params (HitPlayer :type "Actor Object Reference"))
  (locals (HitActor :type "Actor Object Reference"))
  (set `local.HitActor` HitPlayer)
  (switch `/Game/_Main/AI/EAI_AttackTypes` (`self.AttackTypes`)
    (:`NewEnumerator0`
      (`GameplayStatics.ApplyDamage` (`local.HitActor`) (`self.LightAttackDamage`) null self "/Script/Engine.DamageType"))
    (:`NewEnumerator1`
      (`GameplayStatics.ApplyDamage` (`local.HitActor`) (`self.HeavyAttackDamage`) null self "/Script/Engine.DamageType"))
    (:`NewEnumerator2`
      (`GameplayStatics.ApplyDamage` (`local.HitActor`) (`self.RangedAttackDamage`) null self))
    (:`NewEnumerator3`
      (`GameplayStatics.ApplyDamage` (`local.HitActor`) (`self.SpecialAttackDamage`) null self "/Script/Engine.DamageType"))))

(fn `F Percentage`
  (params (Percent :type "Float (double-precision)"))
  (returns (Return :type Boolean))
  (return (select `bool` (== Percent 0.0) :`false` (<= (`KismetMathLibrary.RandomFloatInRange` 0.0 100.0) Percent))))

(fn `F_DistanceCheck`
  (bind _returnvalue (`self.GetDistanceTo` self (`self.PlayerTarget`)))
  (`KismetSystemLibrary.PrintString` (`KismetStringLibrary.Conv_DoubleToString` _returnvalue))
  (if (>= _returnvalue 1500.0)
    (`self.ClearTarget`)
    (`KismetSystemLibrary.K2_ClearAndInvalidateTimerHandle` (`self.DistanceHandle`))))

(fn `F_GetAttackType`
  (returns (AttackTypes :type "/Game/_Main/AI/EAI_AttackTypes Enum"))
  (return (`self.AttackTypes`)))

(fn `F_GetCombatState`
  (returns (InCombat :type Boolean))
  (return (`self.InCombat`)))

(fn `F_GetMontage`
  (params (Montages :type "Array of AnimMontage Object Reference"))
  (returns (Output :type "AnimMontage Object Reference"))
  (return (`|GetArrayItem` Montages (`KismetMathLibrary.RandomIntegerInRange` 0 (- (`KismetArrayLibrary.Array_Length` Montages) 1)))))

(fn `F_GetPlayerTarget`
  (returns (PlayerTarget :type "Actor Object Reference"))
  (return (`self.PlayerTarget`)))

(fn `F_MovementState`
  (params (State :type "/Game/_Main/AI/EAI_MovementState Enum" :default "NewEnumerator0"))
  (bind _walkspeed (`self.WalkSpeed`))
  (set `CharacterMovementComponent.MaxWalkSpeed` (select `/Game/_Main/AI/EAI_MovementState` State :`NewEnumerator1` _walkspeed :`NewEnumerator2` (* _walkspeed (`self.SpeedMultiplier`))) (`self.CharacterMovement`)))

(fn `F_PickAttack`
  (params (DistanceToPlayer :type "Float (double-precision)"))
  (returns (Length :type "Float (double-precision)"))
  (bind _output (`self.F_GetMontage` (`self.RangedAttackMontages`)))
  (bind _output_2 (`self.F_GetMontage` (`self.SpecialAttackMontages`)))
  (bind _output_3 (`self.F_GetMontage` (`self.HeavyAttackMontages`)))
  (bind _output_4 (`self.F_GetMontage` (`self.LightAttackMontages`)))
  (if (<= DistanceToPlayer (`self.MeleeDistance`))
    (if (`self.F Percentage` 70.0)
      (set `self.AttackTypes` "NewEnumerator0")
      (`self.Multi_PlayMontage` (`self.Mesh`) _output_4)
      (bind _returnvalue (`AnimSequenceBase.GetPlayLength` _output_4))
      (return _returnvalue)
      (else
        (set `self.AttackTypes` "NewEnumerator1")
        (`self.Multi_PlayMontage` (`self.Mesh`) _output_3)
        (bind _returnvalue_2 (`AnimSequenceBase.GetPlayLength` _output_3))
        (return _returnvalue_2)))
    (elif (<= DistanceToPlayer (`self.RangedDistance`))
      (set `self.AttackTypes` "NewEnumerator3")
      (`self.Multi_PlayMontage` (`self.Mesh`) _output_2)
      (bind _returnvalue_3 (`AnimSequenceBase.GetPlayLength` _output_2))
      (return _returnvalue_3)
      (else
        (set `self.AttackTypes` "NewEnumerator2")
        (`self.Multi_PlayMontage` (`self.Mesh`) _output)
        (bind _returnvalue_4 (`AnimSequenceBase.GetPlayLength` _output))
        (return _returnvalue_4)))))

(fn `F_PlayDeathAnim`)

(fn `UserConstructionScript`
  (`parent.UserConstructionScript`))