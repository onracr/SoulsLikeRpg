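; Player lock-on targeting component that toggles camera lock onto the nearest living enemy.
; A sphere overlap around the player pawn gathers BP_EnemyBase actors, skips dead ones and picks the closest.
; Message calls lock the player's camera and toggle the enemy's target widget, while a looping timer releases the lock when the target moves out of range.
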(event `Initialize`
  (bind _aspawn (cast `Pawn` (`self.GetOwner`)))
  (bind _output_get (set `self.PlayerPawn` _aspawn))
  (bind _asplayer_controller (cast `PlayerController` (`Pawn.GetController` _output_get)))
  (set `self.PlayerController` _asplayer_controller))

(event `LockOnTarget`
  (if (not (`self.CurrentlyTargeting`))
    (`self.FindTargets`)
    (else
      (`self.ToogleCameraLock` false))))

(event `FindTargets`
  (bind _outactors (`KismetSystemLibrary.SphereOverlapActors` (`Actor.K2_GetActorLocation` (`self.PlayerPawn`)) 1200.0 (`|MakeArray` "ObjectTypeQuery3" :!type "EObjectTypeQuery Enum") "/Game/_Main/AI/BP_EnemyBase.BP_EnemyBase_C"))
  (for _array_element _outactors
    (bind _isdead (message `/Game/_Main/Interfaces/BPI_EnemyAI.IsEnemyDead` _array_element))
    (if (not _isdead)
      (`KismetArrayLibrary.Array_AddUnique` (`self.PotentialTargets`) _array_element)))
  (for _array_element_2 (`self.PotentialTargets`)
    (bind _returnvalue (`Actor.GetDistanceTo` (`self.PlayerPawn`) _array_element_2))
    (if (< _returnvalue (`self.ClosestEnemy`))
      (set `self.ClosestEnemy` _returnvalue)
      (set `self.LockedTarget` _array_element_2)))
  (set `self.ClosestEnemy` 1500.0)
  (`KismetArrayLibrary.Array_Clear` (`self.PotentialTargets`))
  (`self.LockedTarget`
    (:`then`
      (set `self.CurrentlyTargeting` true)
      (`self.ToogleCameraLock` true)
      (bind _returnvalue_2 (`KismetSystemLibrary.K2_SetTimerDelegate` (delegate `CheckTargetDistance`) 0.25 true))
      (set `self.LockHandle` _returnvalue_2))
    (:`else`)))

(event `CheckTargetDistance`
  (if (> (`Actor.GetDistanceTo` (`self.PlayerPawn`) (`self.LockedTarget`)) 1500.0)
    (`self.ToogleCameraLock` false)
    (`KismetSystemLibrary.K2_ClearAndInvalidateTimerHandle` (`self.LockHandle`))))

(event `ToogleCameraLock`
  (params (State :type Boolean))
  (bind _returnvalue (`self.GetOwner`))
  (bind _lockedtarget (`self.LockedTarget`))
  (bind _lockedtarget_2 (`self.LockedTarget`))
  (bind _playerpawn (`self.PlayerPawn`))
  (if State
    (set `self.CurrentlyTargeting` true)
    (message `/Game/_Main/Interfaces/BPI_HeroCharacter.LockCamera` _playerpawn true _lockedtarget_2)
    (message `/Game/_Main/Interfaces/BPI_EnemyAI.ToggleTargetWidget` _lockedtarget true _returnvalue)
    (else
      (set `self.CurrentlyTargeting` false)
      (message `/Game/_Main/Interfaces/BPI_HeroCharacter.LockCamera` _playerpawn false _lockedtarget_2)
      (message `/Game/_Main/Interfaces/BPI_EnemyAI.ToggleTargetWidget` _lockedtarget false _returnvalue)
      (set `self.LockedTarget` null))))