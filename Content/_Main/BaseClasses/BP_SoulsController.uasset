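; BP_SoulsController is the player controller that manages the player's HUD and death screen.
; After a short BeginPlay delay, it creates WBP_PlayerUI for the local controller only and adds it to the viewport.
; Public events relay to client-side events that show pickup messages and update the health bar on that widget.
; On death, the client-side event removes all widgets and displays WBP_DeathScreen.
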(event `self.ReceiveBeginPlay`
  (`KismetSystemLibrary.Delay` 0.2)
  (if (`self.IsLocalPlayerController`)
    (bind _returnvalue (`|CreateWidget` "/Game/_Main/UI/WBP_PlayerUI.WBP_PlayerUI_C"))
    (bind _output_get (set `self.PlayerUI` _returnvalue))
    (`UserWidget.AddToViewport` _output_get 0)))

(event `Client_ShowPickupName`
  (params (Message :type Text) (State :type Boolean))
  (`/Game/_Main/UI/WBP_PlayerUI.PlayerMessage` (`self.PlayerUI`) State Message))

(event `/Game/_Main/Interfaces/BPI_SoulsController.ShowPickupName`
  (params (Name :type Text) (State :type Boolean))
  (`self.Client_ShowPickupName` Name State))

(event `/Game/_Main/Interfaces/BPI_SoulsController.UpdateHealthUI`
  (params (NewHealth :type "Float (single-precision)"))
  (`self.Client_UpdateHealthUI` NewHealth))

(event `Client_UpdateHealthUI`
  (params (Health :type "Float (double-precision)"))
  (`/Game/_Main/UI/WBP_PlayerUI.UpdateHealthBar` (`self.PlayerUI`) Health))

(event `/Game/_Main/Interfaces/BPI_SoulsController.DeathScreenUI`
  (`self.Client_CreateDeathScreen`))

(event `Client_CreateDeathScreen`
  (`WidgetLayoutLibrary.RemoveAllWidgets`)
  (bind _returnvalue (`|CreateWidget` "/Game/_Main/UI/WBP_DeathScreen.WBP_DeathScreen_C"))
  (`UserWidget.AddToViewport` _returnvalue 0))

(fn `UserConstructionScript`)